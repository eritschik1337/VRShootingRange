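; Enemy pawn that relentlessly pursues the player's VRPawn and is destroyed when its health runs out.
; BeginPlay caches the player pawn, starts the chase and picks a random walk speed from the first three of four options, as RandomInteger(3) never selects the last.
; The chase event re-issues AIMoveTo on success or failure, forming an endless follow loop.
; AnyDamage subtracts from clamped Health and destroys the actor at zero.
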(event Custom|Chase%20VRPawn
  (params (VRPawn%20to%20chase :type VR%20Pawn%20Object%20Reference))
  (AI|AIMoveTo self "0, 0, 0" VRPawn%20to%20chase 5.0 false
    (:OnSuccess
      _)
    (:OnFail
      _))
  (CallFunction|ChaseVRPawn (Variables|Default|GetVRPawn%20REF)))

(event EventBeginPlay
  (bind _asvrpawn (Utilities|Casting|CastToVRPawn (Game|Player|GetPlayerPawn 0)))
  (bind _output_get (Variables|Default|SetVRPawn%20REF _asvrpawn))
  (CallFunction|ChaseVRPawn _output_get)
  (Variables|/Script/Engine.CharacterMovementComponent|SetMaxWalkSpeed (Variables|Character|GetCharacterMovement) (Utilities|Select :Index (Math|Random|RandomInteger 3) :Option%200 5e+01 :Option%201 25.0 :Option%202 1e+01 :Option%203 5.0)))

(event Game|Damage|EventAnyDamage
  (params (Damage :type Float%20%28single-precision%29) (DamageType :type Damage%20Type%20Object%20Reference) (InstigatedBy :type Controller%20Object%20Reference) (DamageCauser :type Actor%20Object%20Reference))
  (bind _output_get (Variables|Default|SetHealth (Math|Float|Clamp(Float) (- (Variables|Default|GetHealth) Damage) 0.0 1e+02)))
  (if (== _output_get 0.0)
    (Actor|DestroyActor self)))

(fn ConstructionScript)
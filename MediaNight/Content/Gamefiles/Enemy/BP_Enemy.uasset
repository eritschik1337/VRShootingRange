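; BP_Enemy is a VR enemy character that endlessly chases the player pawn at a randomly picked walk speed.
; ChasePlayer re-issues AIMoveTo on success or failure until death.
; Damage plays an explosion sound and random hit montage, pausing movement until it ends.
; At zero health it disables collision, plays a death montage, increments the player's Kills and destroys itself; RandomInteger(3) never selects each fourth speed or montage option.
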(event Custom|Chase%20Player
  (params (Player%20To%20Chase :type VR%20Pawn%20Object%20Reference))
  (if (not (Variables|Default|GetisDead))
    (AI|AIMoveTo self "0, 0, 0" Player%20To%20Chase 5.0 false
      (:OnSuccess
        _)
      (:OnFail
        _))
    (CallFunction|ChasePlayer (Variables|Default|GetChar%20REF))))

(event EventBeginPlay
  (bind _asvrpawn (Utilities|Casting|CastToVRPawn (Game|Player|GetPlayerPawn 0)))
  (bind _output_get (Variables|Default|SetChar%20REF _asvrpawn))
  (CallFunction|ChasePlayer _output_get)
  (Variables|/Script/Engine.CharacterMovementComponent|SetMaxWalkSpeed (Variables|Character|GetCharacterMovement) (Utilities|Select :Index (Math|Random|RandomInteger 3) :Option%200 2e+02 :Option%201 2.5e+02 :Option%202 3e+02 :Option%203 3.5e+02)))

(event Game|Damage|EventAnyDamage
  (params (Damage :type Float%20%28single-precision%29) (DamageType :type Damage%20Type%20Object%20Reference) (InstigatedBy :type Controller%20Object%20Reference) (DamageCauser :type Actor%20Object%20Reference))
  (bind _returnvalue (Transformation|GetActorLocation))
  (if (not (Variables|Default|GetisDead))
    (bind _output_get (Variables|Default|SetHealth (Math|Float|Clamp(Float) (- (Variables|Default|GetHealth) Damage) 0.0 1e+02)))
    (if (== _output_get 0.0)
      (Audio|PlaySoundatLocation "/Game/StarterContent/Audio/Explosion_Cue.Explosion_Cue" _returnvalue "0, 0, 0" 1.0 1.0 0.0 0 0 0 0)
      (Pawn|Components|CharacterMovement|DisableMovement (Variables|Character|GetCharacterMovement))
      (Variables|Default|SetisDead true)
      (bind _returnvalue_2 (Animation|PlayAnimMontage (Utilities|Select :Index (Math|Random|RandomInteger 3) :Option%200 "/Game/Gamefiles/Enemy/Animations/Death_1_Montage.Death_1_Montage" :Option%201 "/Game/Gamefiles/Enemy/Animations/Death_2_Montage.Death_2_Montage" :Option%202 "/Game/Gamefiles/Enemy/Animations/Death_3_Montage.Death_3_Montage" :Option%203 "/Game/Gamefiles/Enemy/Animations/Death_4_Montage.Death_4_Montage") 1.0 "None"))
      (Collision|SetCollisionEnabled (Variables|Collision|GetCapsuleComponent) "NoCollision")
      (Utilities|FlowControl|Sequence
        (:then_0
          (bind _asvrpawn (Utilities|Casting|CastToVRPawn (Game|Player|GetPlayerPawn 0)))
          (Math|Integer|IncrementInt (Variables|/Game/VRTemplate/Blueprints/VRPawn.VRPawn_C|GetKills _asvrpawn)))
        (:then_1
          (Utilities|FlowControl|Delay _returnvalue_2)
          (Actor|DestroyActor)))
      (else
        (Audio|PlaySoundatLocation "/Game/StarterContent/Audio/Explosion_Cue.Explosion_Cue" _returnvalue "0, 0, 0" 1.0 1.0 0.0 0 0 0 0)
        (Pawn|Components|CharacterMovement|DisableMovement (Variables|Character|GetCharacterMovement))
        (bind _returnvalue_3 (Animation|PlayAnimMontage (Utilities|Select :Index (Math|Random|RandomInteger 3) :Option%200 "/Game/Gamefiles/Enemy/Animations/Hit_1_Montage.Hit_1_Montage" :Option%201 "/Game/Gamefiles/Enemy/Animations/Hit_2_Montage.Hit_2_Montage" :Option%202 "/Game/Gamefiles/Enemy/Animations/Hit_3_Montage.Hit_3_Montage" :Option%203 "/Game/Gamefiles/Enemy/Animations/Hit_4_Montage.Hit_4_Montage") 1.0 "None"))
        (Utilities|FlowControl|Delay _returnvalue_3)
        (if (not (Variables|Default|GetisDead))
          (Pawn|Components|CharacterMovement|SetMovementMode (Variables|Character|GetCharacterMovement) "MOVE_Walking" 0))))))

(fn ConstructionScript)
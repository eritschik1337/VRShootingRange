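; BP_EnemyVR is an enemy that chases the player's VRPawn and is destroyed when shot.
; On BeginPlay it caches the first player pawn as VRPawn and starts an AI MoveTo toward it.
; The chase event calls itself again on either success or failure, so pursuit never stops.
; A component hit on the mesh from a Projectile destroys the enemy.
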(event OnComponentHit(Mesh)
  (params (HitComponent :type Primitive%20Component%20Object%20Reference) (OtherActor :type Actor%20Object%20Reference) (OtherComp :type Primitive%20Component%20Object%20Reference) (NormalImpulse :type Vector :default "0, 0, 0") (Hit :type Hit%20Result%20Structure%20%28by%20ref%29))
  (Utilities|Casting|CastToProjectile OtherActor)
  (Actor|DestroyActor))

(event Custom|chase%20Player
  (params (Player%20to%20chase :type VR%20Pawn%20Object%20Reference))
  (AI|AIMoveTo self "0, 0, 0" Player%20to%20chase 5.0 false
    (:OnSuccess
      _)
    (:OnFail
      _))
  (CallFunction|ChasePlayer (Variables|Default|GetAs%20VRPawn)))

(event EventBeginPlay
  (bind _asvrpawn (Utilities|Casting|CastToVRPawn (Game|Player|GetPlayerPawn 0)))
  (bind _output_get (Variables|Default|SetAs%20VRPawn _asvrpawn))
  (CallFunction|ChasePlayer _output_get))

(fn ConstructionScript)
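; Walking enemy character that endlessly chases the player's VR pawn.
; On BeginPlay it caches the player pawn as a VRPawn, starts the chase and picks a random max walk speed from preset options, though the random range never reaches the fastest one.
; ChasePlayer runs AI MoveTo toward that pawn and calls itself again on success or failure, forming a continuous pursuit loop.
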(event Custom|Chase%20Player
  (params (PlayerToChase :type VR%20Pawn%20Object%20Reference))
  (AI|AIMoveTo self "0, 0, 0" PlayerToChase 5.0 false
    (:OnSuccess
      _)
    (:OnFail
      _))
  (CallFunction|ChasePlayer (Variables|Default|GetChar%20REF)))

(event EventBeginPlay
  (bind _asvrpawn (Utilities|Casting|CastToVRPawn (Game|Player|GetPlayerPawn 0)))
  (bind _output_get (Variables|Default|SetChar%20REF _asvrpawn))
  (CallFunction|ChasePlayer _output_get)
  (Variables|/Script/Engine.CharacterMovementComponent|SetMaxWalkSpeed (Variables|Character|GetCharacterMovement) (Utilities|Select :Index (Math|Random|RandomInteger 3) :Option%200 2e+02 :Option%201 2.5e+02 :Option%202 3e+02 :Option%203 3.5e+02)))

(fn ConstructionScript)